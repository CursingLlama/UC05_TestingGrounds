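; AI controller for guard NPCs that starts the guard behavior tree and its patrol blackboard, then feeds perception results into it.
; Perception updates skip actors tagged "Guard" and branch on sight or hearing by matching the sense class display name.
; Seen actors become the blackboard Enemy.
; Losing sight clears Enemy and, like hearing stimuli, records the stimulus location as the Suspicious Point.
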(event OnTargetPerceptionUpdated(AIPerception)
  (params (Actor :type Actor%20Object%20Reference) (Stimulus :type AI%20Stimulus%20Structure))
  (bind (_age _expirationage _strength _stimuluslocation _receiverlocation _tag _bsuccessfullysensed) (Utilities|Struct|BreakAIStimulus Stimulus))
  (bind _returnvalue (Utilities|Name|MakeLiteralName "Enemy"))
  (bind _blackboard_ref (Variables|Default|GetBlackboard%20Ref))
  (Utilities|IsGuard Actor
    (:False
      (Utilities|BranchbySense Stimulus
        (:AISense_Sight
          (if _bsuccessfullysensed
            (AI|Components|Blackboard|SetValueasObject _blackboard_ref _returnvalue Actor)
            (else
              (AI|Components|Blackboard|ClearValue _blackboard_ref _returnvalue)
              (CallFunction|SetSuspiciousPoint _stimuluslocation :!label _label))))
        (:AISense_Hearing
          (goto _label))))))

(event EventBeginPlay
  ;[1 1 1] Setup Blackboard/Behavior tree
  (bind _blackboardcomponent (Class|AIController|UseBlackboard "/Game/Dynamic/Character/AI/BB_PatrolData.BB_PatrolData"))
  (AI|RunBehaviorTree "/Game/Dynamic/Character/AI/BT_GuardBehavior.BT_GuardBehavior")
  (Variables|Default|SetBlackboard%20Ref _blackboardcomponent))

(event EventTick
  (params (DeltaSeconds :type Float%20%28single-precision%29)))

(fn ConstructionScript)

(fn SetSuspiciousPoint
  (params (VectorValue :type Vector))
  (AI|Components|Blackboard|SetValueasVector (Variables|Default|GetBlackboard%20Ref) (Utilities|Name|MakeLiteralName "Suspicious Point") VectorValue))