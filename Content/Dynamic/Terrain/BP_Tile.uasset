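; Terrain tile for an infinite-terrain mode that scatters props on begin play and gates the player with a barrier.
; The barrier starts red and solid, turns green and passable while the player overlaps LockingVolume, then relocks on exit as the game mode spawns a new tile.
; An Arrow supplies the attach transform, and DestroyVolume destroys the actor when the player enters it.
; PlaceActors calls run from largest to smallest radius, varying rock scale.
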(event OnComponentEndOverlap(LockingVolume)
  (params (OverlappedComponent :type Primitive%20Component%20Object%20Reference) (OtherActor :type Actor%20Object%20Reference) (OtherComp :type Primitive%20Component%20Object%20Reference) (OtherBodyIndex :type Integer))
  ;[1 1 1] Enter/Leave tile
  (Utilities|IsPlayerActor OtherActor
    (:True
      (CallFunction|Lock)
      (bind _asinfinite_terrain_game_mode (Utilities|Casting|CastToInfiniteTerrainGameMode (Game|GetGameMode)))
      (Default|SpawnNewTile _asinfinite_terrain_game_mode))))

(event OnComponentBeginOverlap(DestroyVolume)
  (params (OverlappedComponent :type Primitive%20Component%20Object%20Reference) (OtherActor :type Actor%20Object%20Reference) (OtherComp :type Primitive%20Component%20Object%20Reference) (OtherBodyIndex :type Integer) (bFromSweep :type Boolean) (SweepResult :type Hit%20Result%20Structure%20%28by%20ref%29))
  (Utilities|IsPlayerActor OtherActor
    (:True
      (Actor|DestroyActor))))

(event OnComponentBeginOverlap(LockingVolume)
  (params (OverlappedComponent :type Primitive%20Component%20Object%20Reference) (OtherActor :type Actor%20Object%20Reference) (OtherComp :type Primitive%20Component%20Object%20Reference) (OtherBodyIndex :type Integer) (bFromSweep :type Boolean) (SweepResult :type Hit%20Result%20Structure%20%28by%20ref%29))
  ;[1 1 1] Enter/Leave tile
  (Utilities|IsPlayerActor OtherActor
    (:True
      (CallFunction|Unlock))))

(event EventBeginPlay
  (CallFunction|Lock)
  (Class|Tile|PlaceActors "/Game/Dynamic/Terrain/Props/BP_CargoContainer_Open.BP_CargoContainer_Open_C" 0 1 475.0 1.0 1.0)
  (Class|Tile|PlaceActors "/Game/Dynamic/Terrain/Props/BP_CargoContainer_Closed.BP_CargoContainer_Closed_C" 0 2 425.0 1.0 1.0)
  (Class|Tile|PlaceActors "/Game/Dynamic/Terrain/Props/BP_Rock02.BP_Rock02_C" 0 4 2.6e+02 0.25 2.5)
  (Class|Tile|PlaceActors "/Game/Dynamic/Terrain/Props/BP_Rock03.BP_Rock03_C" 0 4 2.5e+02 0.25 2.5)
  (Class|Tile|PlaceActors "/Game/Dynamic/Terrain/Props/BP_Rock01.BP_Rock01_C" 0 4 175.0 0.25 2.5)
  (Class|Tile|PlaceActors "/Game/Dynamic/Terrain/Props/BP_SandbagWall.BP_SandbagWall_C" 0 2 145.0 1.0 1.0)
  (Class|Tile|PlaceActors "/Game/Dynamic/Terrain/Props/BP_Crate.BP_Crate_C" 0 5 125.0 1.0 1.0)
  (Class|Tile|PlaceActors "/Game/Dynamic/Terrain/Props/BP_Canister.BP_Canister_C" 0 4 85.0 1.0 1.0))

(event Collision|EventActorBeginOverlap
  (params (OtherActor :type Actor%20Object%20Reference)))

(event EventTick
  (params (DeltaSeconds :type Float%20%28single-precision%29)))

(fn ConstructionScript)

(fn GetAttachLocation
  (return (Transformation|GetWorldTransform (Variables|Default|GetArrow))))

(fn Unlock
  (bind _barrier (Variables|Default|GetBarrier))
  (Collision|SetCollisionEnabled _barrier "NoCollision")
  (Rendering|Material|SetMaterial _barrier 0 "/Game/Dynamic/Terrain/MI_Barrier_Green.MI_Barrier_Green"))

(fn Lock
  (bind _barrier (Variables|Default|GetBarrier))
  (Collision|SetCollisionEnabled _barrier "QueryAndPhysics")
  (Rendering|Material|SetMaterial _barrier 0 "/Game/Dynamic/Terrain/MI_Barrier_Red.MI_Barrier_Red"))