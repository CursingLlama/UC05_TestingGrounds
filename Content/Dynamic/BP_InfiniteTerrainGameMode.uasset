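; Game mode for an infinite terrain game that builds the level from BP_Tile actors and keeps score of conquered tiles.
; On BeginPlay it populates a bounds volume pool and spawns the starting run of tiles.
; Each new tile receives the nav mesh pool and its attach location becomes the next spawn point, chaining tiles end to end.
; NewTileConquered increments the score.
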(event EventBeginPlay
  (Class|InfiniteTerrainGameMode|PopulateBoundsVolumePool)
  (for _index (range 0 3)
    (CallFunction|SpawnNewTile)))

(event EventTick
  (params (DeltaSeconds :type Float%20%28single-precision%29)))

(fn ConstructionScript)

(fn SpawnNewTile
  (bind _returnvalue (Game|SpawnActorfromClass "/Game/Dynamic/Terrain/BP_Tile.BP_Tile_C" (Variables|Default|GetTile%20Spawn%20Point) "Undefined" 0 0))
  (Class|Tile|SetPool _returnvalue (Variables|Default|GetNavMeshPool))
  (bind _attachment_point (Default|GetAttachLocation _returnvalue))
  (Variables|Default|SetTile%20Spawn%20Point _attachment_point))

(fn NewTileConquered
  (Math|Integer|IncrementInt (Variables|Default|GetScore)))