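; AI controller Blueprint for guard NPCs that runs the GuardBehavior tree on the PatrolData blackboard.
; Perception updates feed that blackboard, ignoring any actor tagged Guard.
; A sighted actor becomes the Focus Point; losing sight clears it and records the stimulus location as the Suspicious Point.
; Heard stimuli also set the Suspicious Point, with senses told apart by class display name.
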(event OnTargetPerceptionUpdated(AIPerception)
  (params (Actor :type Actor%20Object%20Reference) (Stimulus :type AI%20Stimulus%20Structure))
  (bind (_age _expirationage _strength _stimuluslocation _receiverlocation _tag _bsuccessfullysensed) (Utilities|Struct|BreakAIStimulus Stimulus))
  (bind _returnvalue (Utilities|Name|MakeLiteralName "Focus Point"))
  (bind _blackboard_ref (Variables|Default|GetBlackboard%20Ref))
  (if (not (Actor|ActorHasTag Actor "Guard"))
    (bind _returnvalue_2 (Class|AIPerceptionSystem|GetSenseClassforStimulus Stimulus))
    (switch string (Utilities|GetClassDisplayName _returnvalue_2)
      (:AISense_Sight
        (if _bsuccessfullysensed
          (AI|Components|Blackboard|SetValueasObject _blackboard_ref _returnvalue Actor)
          (else
            (AI|Components|Blackboard|ClearValue _blackboard_ref _returnvalue)
            (AI|Components|Blackboard|SetValueasVector (Variables|Default|GetBlackboard%20Ref) (Utilities|Name|MakeLiteralName "Suspicious Point") _stimuluslocation :!label _label))))
      (:AISense_Hearing
        (goto _label)))))

(event EventBeginPlay
  (bind _blackboardcomponent (Class|AIController|UseBlackboard "/Game/Dynamic/NPC/AI/PatrolData.PatrolData"))
  (AI|RunBehaviorTree "/Game/Dynamic/NPC/AI/GuardBehavior.GuardBehavior")
  (Variables|Default|SetBlackboard%20Ref _blackboardcomponent))

(event EventTick
  (params (DeltaSeconds :type Float%20%28single-precision%29)))

(fn ConstructionScript)